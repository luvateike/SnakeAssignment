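; BP_Tail_BACKUP is a tail actor owned by a player that kills any other BP_Player overlapping it.
; Overlap casts to BP_Player and calls Die unless that player is PlayerOwner.
; Tick applies the Color material to the Sphere once it is valid, guarded by a HasSetMaterial flag.
; A Tick-driven timer periodically checks PlayerOwner and destroys the tail when the owner is no longer valid.
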(event `self.ReceiveActorBeginOverlap`
  (params (OtherActor :type "Actor Object Reference"))
  (bind _asbp_player (cast `/Game/Blueprints/BP_Player` OtherActor))
  (if (not (== _asbp_player (`self.PlayerOwner`)))
    (`SCR_Player.Die` _asbp_player)))

(event `self.ReceiveTick`
  (params (DeltaSeconds :type "Float (single-precision)"))
  (bind _timer (`self.timer`))
  (bind _sphere (`self.Sphere`))
  (bind _color (`self.Color`))
  (`|ExecutionSequence`
    (:`then_0`
      (if (`self.hasSetMaterial`)
        _
        (elif (and (!= (`PrimitiveComponent.GetMaterial` _sphere 0) _color) (`KismetSystemLibrary.IsValid` _color))
          (`PrimitiveComponent.SetMaterial` _sphere 0 _color)
          (set `self.hasSetMaterial` true))))
    (:`then_1`
      (if (> _timer 0.2)
        (set `self.timer` 0.0)
        (if (not (`KismetSystemLibrary.IsValid` (`self.PlayerOwner`)))
          (`self.K2_DestroyActor`))
        (else
          (set `self.timer` (+ _timer DeltaSeconds)))))))

(fn `UserConstructionScript`)