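; BP_Player is a player, human or AI, with a head and a body of BP_Tail segments, colored by who controls it.
; Shortly after BeginPlay it picks a material from the AI flag or player number and applies it to the head.
; Tick rebuilds the typed Tails array whenever its length differs from Body, passing that material to each segment.
; The head's overlap event is empty.
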(event `self.ReceiveBeginPlay`
  (bind _playernumber (`self.playerNumber`))
  (`KismetSystemLibrary.Delay` 0.5)
  (if (`self.bIsAI`)
    (set `self.Color` "/Game/Materials/Yellow.Yellow")
    (elif (== _playernumber -1)
      (set `self.Color` "/Game/Materials/Pink.Pink")
      (else
        (set `self.Color` (`|GetArrayItem` (`self.Colors`) _playernumber)))))
  (`PrimitiveComponent.SetMaterial` (`self.Head`) 0 (`self.Color`)))

(event `self.ReceiveTick`
  (params (DeltaSeconds :type "Float (single-precision)"))
  (if (and (!= (`KismetArrayLibrary.Array_Length` (`self.Body`)) (`KismetArrayLibrary.Array_Length` (`self.Tails`))) (`KismetSystemLibrary.IsValid` (`self.Color`)))
    (`|ExecutionSequence`
      (:`then_0`
        (`KismetArrayLibrary.Array_Clear` (`self.Tails`)))
      (:`then_1`
        (for _array_element (`self.Body`)
          (bind _asbp_tail (cast `/Game/Blueprints/BP_Tail` _array_element))
          (`KismetArrayLibrary.Array_Add` (`self.Tails`) _asbp_tail)
          (set `/Game/Blueprints/BP_Tail.Color` (`self.Color`) _asbp_tail))))))

(event `self.HeadCollision.OnComponentBeginOverlap`
  (params (OverlappedComponent :type "PrimitiveComponent Object Reference") (OtherActor :type "Actor Object Reference") (OtherComp :type "PrimitiveComponent Object Reference") (OtherBodyIndex :type Integer) (bFromSweep :type Boolean) (SweepResult :type "HitResult Structure (by ref)")))

(fn `UserConstructionScript`)